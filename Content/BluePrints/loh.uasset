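; Damageable character, apparently an enemy, that raises the player's rage when hit and plays hit-react or death montages.
; AnyDamage passes a DoOnce, adds rage on the cached CHAR_Player, then calls FUNCHP, which subtracts armor-divided damage from HP.
; The stored damage is not passed to FUNCHP, whose input is zero.
; The gate resets after the hit-react montage; at zero HP the actor is destroyed after the death montage.
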(event `self.ReceiveBeginPlay`
  ;[0.078 1 0] Инициализация
  (bind _aschar_player (cast `/Game/BluePrints/CHAR_Player` (`GameplayStatics.GetPlayerCharacter` 0)))
  (set `self.As CHAR Player` _aschar_player))

(event `self.ReceiveAnyDamage`
  (params (Damage :type "Float (single-precision)") (DamageType :type "DamageType Object Reference") (InstigatedBy :type "Controller Object Reference") (DamageCauser :type "Actor Object Reference"))
  ;[1 1 0] Получаем урон
  (set `self.REV_DAMAGE` Damage)
  (`/Engine/EditorBlueprintResources/StandardMacros.DoOnce` false :!label _label
    (:`Completed`
      (`/Game/BluePrints/CHAR_Player.FUNC_RAGE_UP` (`self.As CHAR Player`) 10.0)
      (bind _output_get (`self.FUNC_HP` 0.0))
      (if (<= _output_get 0.0)
        ;;[1 1 0] Смерть
        (bind _returnvalue (`self.PlayAnimMontage` "/Game/BluePrints/Player/Death_Montage.Death_Montage"))
        (`KismetSystemLibrary.Delay` _returnvalue)
        (`self.K2_DestroyActor`)
        (else
          ;;[1 1 0] Получение урона
          (bind _returnvalue_2 (`self.PlayAnimMontage` "/Game/BluePrints/Player/HitReact_Montage.HitReact_Montage"))
          (`KismetSystemLibrary.Delay` _returnvalue_2)
          (goto _label :!via `Reset`))))))

(fn `FUNC_HP`
  (params (`rev damage` :type "Float (double-precision)"))
  (returns (Output_Get :type "Float (double-precision)"))
  (bind _output_get (set `self.HP` (- (`self.HP`) (/ `rev damage` (`self.ARMORE`)))))
  (return _output_get))

(fn `UserConstructionScript`)