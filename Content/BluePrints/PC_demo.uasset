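; PC_demo is a player controller Blueprint that toggles a pause menu on the Open PMenu input.
; A FlipFlop drives game pause and cursor visibility, then either shows or removes the BM widget.
; The widget is created on first use and cached in UIREF, with input switching between Game and UI and Game Only.
; The construction script and Menu Mode Enter function are empty.
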(event `self.ReceiveBeginPlay`
  ;[1 1 1] Инициализация
  (set `self.PC REF` (`GameplayStatics.GetPlayerController` 0)))

(event `InputAction|Open PMenu` :paused true
  (params (Key :type "Key Structure"))
  (:`Pressed`
    (bind _isa (`/Engine/EditorBlueprintResources/StandardMacros.FlipFlop`)
      (:`A`
        _)
      (:`B`
        _))
    (`GameplayStatics.SetGamePaused` _isa)
    (set `self.bShowMouseCursor` _isa)
    (`/Engine/EditorBlueprintResources/StandardMacros.FlipFlop`
      (:`A`
        (`/Engine/EditorBlueprintResources/StandardMacros.IsValid` (`self.UI REF`)
          (:`Is Valid`
            _)
          (:`Is Not Valid`
            (bind _returnvalue (`|CreateWidget` "/Game/BluePrints/UI/BM/BM.BM_C" (`self.PC REF`)))
            (bind _output_get (set `self.UI REF` _returnvalue))))
        (`UserWidget.AddToViewport` _output_get 0)
        (`WidgetBlueprintLibrary.SetInputMode_GameAndUIEx` (`self.PC REF`) (`self.UI REF`) "LockInFullscreen" false))
      (:`B`
        (`Widget.RemoveFromParent` (`self.UI REF`))
        (`WidgetBlueprintLibrary.SetInputMode_GameOnly` (`self.PC REF`))))))

(fn `Menu Mode Enter`
  (params (`Widget?` :type "UserWidget Class Reference"))
  (returns (NewParam :type "Widget Object Reference"))
  (locals (PC_REF :type "PlayerController Object Reference") (`Widget Class REF` :type "UserWidget Class Reference" :default null)))

(fn `UserConstructionScript`)