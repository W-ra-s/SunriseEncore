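; Game instance Blueprint (MGINST) that acts as the central hub for menu UI and game flow.
; Events lazily create, cache and show widgets for the main menu, loading screen, pause menu and in-game inventory, spell, quest and map screens.
; The pause menu toggles game pause, input mode and cursor.
; New game and continue both open the demo level; saving only prints an in-development message.
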(event `MM Show`
  ;[1 1 1] Главное меню
  ;;[0 1 0.5] Вызываем главное меню
  (`/Engine/EditorBlueprintResources/StandardMacros.IsValid` (`self.MM`)
    (:`Is Valid`
      _)
    (:`Is Not Valid`
      (bind _returnvalue (`|CreateWidget` "/Game/BluePrints/UI/MM/MM.MM_C" (`GameplayStatics.GetPlayerController` 0)))
      (bind _output_get (set `self.MM` _returnvalue))))
  (`UserWidget.AddToViewport` _output_get 0))

(event `LS Show`
  (bind _returnvalue (`GameplayStatics.GetPlayerController` 0))
  ;[1 1 1] Окно загрузки
  ;;[0 1 0.5] Вызов окна загркзки
  (set `PlayerController.bShowMouseCursor` false _returnvalue)
  (`/Engine/EditorBlueprintResources/StandardMacros.IsValid` (`self.LoadingScreen`)
    (:`Is Valid`
      _)
    (:`Is Not Valid`
      (bind _returnvalue_2 (`|CreateWidget` "/Game/BluePrints/UI/UIW_LoadScreen.UIW_LoadScreen_C" _returnvalue))
      (bind _output_get (set `self.LoadingScreen` _returnvalue_2))))
  (`UserWidget.AddToViewport` _output_get 0))

(event `PM Show`
  (bind _returnvalue (`GameplayStatics.GetPlayerController` 0))
  ;[1 0 0] BM
  ;;[0 1 0.5] Вызов меню паузы
  (`/Engine/EditorBlueprintResources/StandardMacros.IsValid` (`self.PM`)
    (:`Is Valid`
      _)
    (:`Is Not Valid`
      (bind _returnvalue_2 (`|CreateWidget` "/Game/BluePrints/UI/BP/BM_PM.BM_PM_C" _returnvalue))
      (bind _output_get (set `self.PM` _returnvalue_2))))
  (`UserWidget.AddToViewport` _output_get 0)
  (`WidgetBlueprintLibrary.SetInputMode_UIOnlyEx` _returnvalue (`self.PM`) "LockInFullscreen")
  (`GameplayStatics.SetGamePaused` true)
  (set `PlayerController.bShowMouseCursor` true _returnvalue))

(event `MM Creat New Game`
  ;[1 1 1] Главное меню
  ;;[1 0 0] Начало новой игры
  (`GameplayStatics.OpenLevelBySoftObjectPtr` "/Game/Levels/Demo/LVL_Demo.LVL_Demo"))

(event `Exit Game`
  ;[1 1 1] Окно загрузки
  ;;[1 1 1] Выход из игры
  (`KismetSystemLibrary.QuitGame` (`GameplayStatics.GetPlayerController` 0) "Quit"))

(event `LS Remove`
  ;[1 1 1] Окно загрузки
  ;;[1 1 1] Убрать окно загрузки
  (`Widget.RemoveFromParent` (`self.LoadingScreen`)))

(event `BM Inventory Show`
  ;[1 0 0] BM
  ;;[1 1 1] Вызвать меню инвентаря
  (`/Engine/EditorBlueprintResources/StandardMacros.IsValid` (`self.BM Inventory`)
    (:`Is Valid`
      _)
    (:`Is Not Valid`
      (bind _returnvalue (`|CreateWidget` "/Game/BluePrints/UI/BP/BM_Inventory.BM_Inventory_C" (`GameplayStatics.GetPlayerController` 0)))
      (bind _output_get (set `self.BM Inventory` _returnvalue))))
  (`UserWidget.AddToViewport` _output_get 0))

(event `PM Resume`
  (bind _returnvalue (`GameplayStatics.GetPlayerController` 0))
  ;[1 0 0] BM
  ;;[1 1 1] PM
  ;;;[1 1 1] Вернуться в игру из меню паузы
  (`Widget.RemoveFromParent` (`self.PM`))
  (`WidgetBlueprintLibrary.SetInputMode_GameOnly` _returnvalue)
  (set `PlayerController.bShowMouseCursor` false _returnvalue)
  (`GameplayStatics.SetGamePaused` false))

(event `MM Resume Game`
  ;[1 1 1] Главное меню
  ;;[1 0 0] Продолжить игру
  (`GameplayStatics.OpenLevelBySoftObjectPtr` "/Game/Levels/Demo/LVL_Demo.LVL_Demo"))

(event `MM Saves Show`
  ;[1 1 1] Главное меню
  ;;[1 0 1] Вызов меню загрукзок
  (`/Engine/EditorBlueprintResources/StandardMacros.IsValid` (`self.MM Saves`)
    (:`Is Valid`
      _)
    (:`Is Not Valid`
      (bind _returnvalue (`|CreateWidget` "/Game/BluePrints/UI/MM/MM_Saves.MM_Saves_C" (`GameplayStatics.GetPlayerController` 0)))
      (bind _output_get (set `self.MM Saves` _returnvalue))))
  (`UserWidget.AddToViewport` _output_get 0))

(event `BM Spels Show`
  ;[1 0 0] BM
  ;;[1 1 1] Вызвать меню способностей
  (`/Engine/EditorBlueprintResources/StandardMacros.IsValid` (`self.BM Spels`)
    (:`Is Valid`
      _)
    (:`Is Not Valid`
      (bind _returnvalue (`|CreateWidget` "/Game/BluePrints/UI/BP/BM_Spels.BM_Spels_C" (`GameplayStatics.GetPlayerController` 0)))
      (bind _output_get (set `self.BM Spels` _returnvalue))))
  (`UserWidget.AddToViewport` _output_get 0))

(event `PM Save game`
  ;[1 0 0] BM
  ;;[1 1 1] PM
  ;;;[1 1 1] Сохранить игру
  (`KismetSystemLibrary.PrintString` "В разработке" true true (struct :`R` 1.0 :`A` 1.0) 1.0))

(event `PM Loads Show`
  ;[1 0 0] BM
  ;;[1 1 1] PM
  ;;;[1 1 1] Вызов меню загрукзок
  (`/Engine/EditorBlueprintResources/StandardMacros.IsValid` (`self.PM Saves`)
    (:`Is Valid`
      _)
    (:`Is Not Valid`
      (bind _returnvalue (`|CreateWidget` "/Game/BluePrints/UI/PM/PM_Saves.PM_Saves_C" (`GameplayStatics.GetPlayerController` 0)))
      (bind _output_get (set `self.PM Saves` _returnvalue))))
  (`UserWidget.AddToViewport` _output_get 0))

(event `MM Settings Show`
  ;[1 1 1] Главное меню
  ;;[1 0 1] Вызов меню настроек
  (`/Engine/EditorBlueprintResources/StandardMacros.IsValid` (`self.MM Settings`)
    (:`Is Valid`
      _)
    (:`Is Not Valid`
      (bind _returnvalue (`|CreateWidget` "/Game/BluePrints/UI/MM/MM_Settings.MM_Settings_C" (`GameplayStatics.GetPlayerController` 0)))
      (bind _output_get (set `self.MM Settings` _returnvalue))))
  (`UserWidget.AddToViewport` _output_get 0))

(event `BM Quests Show`
  ;[1 0 0] BM
  ;;[1 1 1] Вызвать меню заданий
  (`/Engine/EditorBlueprintResources/StandardMacros.IsValid` (`self.BM Quests`)
    (:`Is Valid`
      _)
    (:`Is Not Valid`
      (bind _returnvalue (`|CreateWidget` "/Game/BluePrints/UI/BP/BM_Quests.BM_Quests_C" (`GameplayStatics.GetPlayerController` 0)))
      (bind _output_get (set `self.BM Quests` _returnvalue))))
  (`UserWidget.AddToViewport` _output_get 0))

(event `PM Settings Show`
  ;[1 0 0] BM
  ;;[1 1 1] PM
  ;;;[1 1 1] Вызвать меню настроек
  (`/Engine/EditorBlueprintResources/StandardMacros.IsValid` (`self.PM Settings`)
    (:`Is Valid`
      _)
    (:`Is Not Valid`
      (bind _returnvalue (`|CreateWidget` "/Game/BluePrints/UI/PM/PM_Settings.PM_Settings_C" (`GameplayStatics.GetPlayerController` 0)))
      (bind _output_get (set `self.PM Settings` _returnvalue))))
  (`UserWidget.AddToViewport` _output_get 0))

(event `BM Map Show`
  ;[1 0 0] BM
  ;;[1 1 1] Вызвать меню карта
  (`/Engine/EditorBlueprintResources/StandardMacros.IsValid` (`self.BM map`)
    (:`Is Valid`
      _)
    (:`Is Not Valid`
      (bind _returnvalue (`|CreateWidget` "/Game/BluePrints/UI/BP/BM_Map.BM_Map_C" (`GameplayStatics.GetPlayerController` 0)))
      (bind _output_get (set `self.BM map` _returnvalue))))
  (`UserWidget.AddToViewport` _output_get 0))

(event `PM Exit`
  ;[1 0 0] BM
  ;;[1 1 1] PM
  ;;;[1 1 1] Вызвать выхода
  (`/Engine/EditorBlueprintResources/StandardMacros.IsValid` (`self.PM Exit quest`)
    (:`Is Valid`
      _)
    (:`Is Not Valid`
      (bind _returnvalue (`|CreateWidget` "/Game/BluePrints/UI/PM/PM_Exit.PM_Exit_C" (`GameplayStatics.GetPlayerController` 0)))
      (bind _output_get (set `self.PM Exit quest` _returnvalue))))
  (`UserWidget.AddToViewport` _output_get 0))